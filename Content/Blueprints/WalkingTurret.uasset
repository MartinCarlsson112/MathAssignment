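; Walking turret actor that poses two front legs with procedural IK and runs a turret that detects and fires.
; BeginPlay builds left and right IK chains from leg bone components and start/end markers.
; Tick refreshes each chain's endpoints from those markers and solves it with FABRIK.
; A short Delay in Tick throttles the Turret's Detect and Fire calls.
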(event `self.ReceiveBeginPlay`
  (bind _returnvalue (`IKSolver.CreateIKChain` (`|MakeArray` (`self.FrontLegLeft1`) (`self.FrontLegLeft2`) (`self.FrontLegLeft7`) (`self.FrontLegLeft3`)) (`SceneComponent.K2_GetComponentLocation` (`self.StartLocationFL`)) (`SceneComponent.K2_GetComponentLocation` (`self.EndLocationFL`))))
  (set `self.FrontLeftLeg` _returnvalue)
  (bind _returnvalue_2 (`IKSolver.CreateIKChain` (`|MakeArray` (`self.FrontLegLeft4`) (`self.FrontLegLeft5`) (`self.FrontLegLeft6`)) (`SceneComponent.K2_GetComponentLocation` (`self.StartLocationFR`)) (`SceneComponent.K2_GetComponentLocation` (`self.EndLocationFR`))))
  (set `self.FrontRightLeg` _returnvalue_2))

(event `self.ReceiveTick`
  (params (DeltaSeconds :type "Float (single-precision)"))
  (bind (_chain _size _totallength) (break `IKChain2` (`self.FrontRightLeg`)))
  (bind (_chain_2 _size_2 _totallength_2) (break `IKChain2` (`self.FrontLeftLeg`)))
  (bind (_out_start_loc _outendloc) (`self.GetStartAndEndLocations` (`self.EndLocationFR`) (`self.StartLocationFR`)))
  (bind (_out_start_loc_2 _outendloc_2) (`self.GetStartAndEndLocations` (`self.EndLocationFL`) (`self.StartLocationFL`)))
  (bind _output_get (set `self.FrontLeftLeg` (make `IKChain2` _chain_2 _size_2 _totallength_2 _outendloc_2 _out_start_loc_2)))
  (`IKSolver.SolveIKChainFABRIK` _output_get)
  (bind _output_get_2 (set `self.FrontRightLeg` (make `IKChain2` _chain _size _totallength _outendloc _out_start_loc)))
  (`IKSolver.SolveIKChainFABRIK` _output_get_2)
  (`KismetSystemLibrary.Delay` 0.1)
  (`/Game/Blueprints/Turret.Detect` (`self.Turret`))
  (`/Game/Blueprints/Turret.Fire` (`self.Turret`)))

(fn `UserConstructionScript`)