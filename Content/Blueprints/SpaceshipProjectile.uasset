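; Spaceship projectile actor that damages whatever it overlaps and then destroys itself.
; OnFired launches it by setting the physics linear velocity of its Sphere from a direction and speed, and stores a maximum lifetime.
; Overlap applies fixed generic damage to the other actor, while Tick destroys the projectile once its age exceeds that lifetime.
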(event `self.ReceiveActorBeginOverlap`
  (params (OtherActor :type "Actor Object Reference"))
  (`GameplayStatics.ApplyDamage` OtherActor 10.0 null null "/Script/Engine.DamageType")
  (`self.K2_DestroyActor` :!label _label))

(event `self.ReceiveTick`
  (params (DeltaSeconds :type "Float (single-precision)"))
  (if (> (`self.GetGameTimeSinceCreation`) (`self.Max Lifetime`))
    (goto _label)))

(fn `OnFired`
  (params (Direction :type "Vector Structure") (Speed :type "Float (double-precision)") (`Max Lifetime` :type "Float (double-precision)"))
  (`PrimitiveComponent.SetPhysicsLinearVelocity` (`self.Sphere`) (* Direction Speed) false "None")
  (set `self.Max Lifetime` `Max Lifetime`))

(fn `UserConstructionScript`)