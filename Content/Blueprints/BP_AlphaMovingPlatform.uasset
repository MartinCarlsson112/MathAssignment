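; BP_AlphaMovingPlatform is a moving platform actor made up of nine orbiting platform components.
; Every Tick, it passes all nine components to OrbitSolveMultiple, whose logic is defined outside this file, to update their orbits.
; BeginPlay, overlap and the construction script do nothing, so that single per-frame call is the only behavior in its graphs.
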(event `self.ReceiveTick`
  (params (DeltaSeconds :type "Float (single-precision)"))
  (`self.OrbitSolveMultiple` (`|MakeArray` (`self.OrbitingPlatform`) (`self.OrbitingPlatform1`) (`self.OrbitingPlatform2`) (`self.OrbitingPlatform3`) (`self.OrbitingPlatform4`) (`self.OrbitingPlatform5`) (`self.OrbitingPlatform6`) (`self.OrbitingPlatform7`) (`self.OrbitingPlatform8`))))

(fn `UserConstructionScript`)