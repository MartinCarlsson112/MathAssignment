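; Player-controlled spaceship that flies on physics, fires projectiles and shows a crosshair.
; Each tick, turn and look input update a pitch-clamped target, which the capsule's rotation eases toward via interpolation and a quaternion.
; Movement axes are rotated into ship space and added to linear velocity, with each increment clamped.
; Shooting launches a projectile along the capsule's negative up vector; received damage lowers Health and prints it.
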(event `InputAction|Shoot`
  (params (Key :type "Key Structure"))
  (bind (_returnvalue_location _returnvalue_rotation) (`KismetMathLibrary.BreakTransform` (`SceneComponent.K2_GetComponentToWorld` (`self.Capsule`))))
  (:`Pressed`
    (bind _returnvalue (`|SpawnActorFromClass` "/Game/Blueprints/SpaceshipProjectile.SpaceshipProjectile_C" (`KismetMathLibrary.MakeTransform` _returnvalue_location _returnvalue_rotation (0.1 0.1 0.1)) "AlwaysSpawn" "OverrideRootScale" null null))
    (`/Engine/EditorBlueprintResources/StandardMacros.IsValid` _returnvalue
      (:`Is Valid`
        (`/Game/Blueprints/SpaceshipProjectile.OnFired` _returnvalue (* (`SceneComponent.GetUpVector` (`self.Capsule`)) -1.0) (`self.Projectile Speed`) 10.0 self)))))

(event `self.ReceiveBeginPlay`
  (bind (_relativerotation_roll _relativerotation_pitch _relativerotation_yaw) (`KismetMathLibrary.BreakRotator` (`SceneComponent.RelativeRotation` (`self.Capsule`))))
  (set `self.Target Look` (`KismetMathLibrary.MakeVector2D` _relativerotation_yaw _relativerotation_pitch))
  (bind _returnvalue (`|CreateWidget` "/Game/Blueprints/Crosshair.Crosshair_C"))
  (`UserWidget.AddToViewport` _returnvalue 0))

(event `self.ReceiveTick`
  (params (DeltaSeconds :type "Float (single-precision)"))
  (bind _capsule (`self.Capsule`))
  (bind _look_sensitivity (`self.Look Sensitivity`))
  (bind (_target_look_x _target_look_y) (`KismetMathLibrary.BreakVector2D` (`self.Target Look`)))
  (bind _look_speed (`self.Look Speed`))
  (bind (_current_direction_x _current_direction_y) (`KismetMathLibrary.BreakVector2D` (`self.Current Direction`)))
  (bind _output_get (set `self.Target Look` (`KismetMathLibrary.MakeVector2D` (+ (* (* (`self.GetInputAxisValue`) _look_sensitivity) DeltaSeconds) _target_look_x) (`KismetMathLibrary.FClamp` (+ (* (* (`self.GetInputAxisValue`) _look_sensitivity) DeltaSeconds) _target_look_y) 0.0 180.0))))
  (bind _output_get_2 (set `self.Current Direction` (`KismetMathLibrary.MakeVector2D` (`KismetMathLibrary.FInterpTo` _current_direction_x (`KismetMathLibrary.BreakVector2D` _output_get) DeltaSeconds _look_speed) (`KismetMathLibrary.FInterpTo` _current_direction_y (`.Y` (`KismetMathLibrary.BreakVector2D` _output_get)) DeltaSeconds _look_speed))))
  (`SceneComponent.K2_SetRelativeRotation` (`self.Capsule`) (`KismetMathLibrary.Quat_Rotator` (`KismetMathLibrary.Quat_MakeFromEuler` (`KismetMathLibrary.MakeVector` 0.0 (`.Y` (`KismetMathLibrary.BreakVector2D` _output_get_2)) (`KismetMathLibrary.BreakVector2D` _output_get_2)))) false false)
  (`PrimitiveComponent.SetPhysicsLinearVelocity` _capsule (`KismetMathLibrary.ClampVectorSize` (* (* (`KismetMathLibrary.GreaterGreater_VectorRotator` (`KismetMathLibrary.Normal` (`KismetMathLibrary.MakeVector` (`self.GetInputAxisValue`) (`self.GetInputAxisValue`) (* (`self.GetInputAxisValue`) -1.0))) (`SceneComponent.RelativeRotation` _capsule)) (`self.Acceleration`)) DeltaSeconds) 0.0 (`self.Maximum Speed`)) true "None"))

(fn `ReceiveDamage`
  (params (DamageAmount :type "Float (double-precision)") (Shooter :type "Actor Object Reference"))
  (returns (DamageDealt :type "Float (double-precision)"))
  (bind _output_get (set `self.Health` (- (`self.Health`) DamageAmount)))
  (`KismetSystemLibrary.PrintString` (`KismetStringLibrary.Concat_StrStr` "Health: " (`KismetStringLibrary.Conv_DoubleToString` _output_get)))
  (return DamageAmount))

(fn `UserConstructionScript`)