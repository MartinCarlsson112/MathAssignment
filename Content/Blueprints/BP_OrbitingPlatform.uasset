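; BP_OrbitingPlatform is an actor with twelve platform components that move in nested orbits.
; Every Tick, OrbitSolveMultiple moves three primary platforms around the default pivot.
; It then solves three groups of three satellites, each using one primary platform's current relative location as its pivot, so orbits chain hierarchically.
; All calls disable VInterp, and the orbit math is defined outside this file.
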(event `self.ReceiveBeginPlay`)

(event `self.ReceiveTick`
  (params (DeltaSeconds :type "Float (single-precision)"))
  (`self.OrbitSolveMultiple` (`|MakeArray` (`self.OrbitingPlatform`) (`self.OrbitingPlatform1`) (`self.OrbitingPlatform2`)) (0.0 0.0 0.0) false)
  (`self.OrbitSolveMultiple` (`|MakeArray` (`self.OrbitingPlatform3`) (`self.OrbitingPlatform4`) (`self.OrbitingPlatform5`)) (`SceneComponent.RelativeLocation` (`self.OrbitingPlatform`)) false)
  (`self.OrbitSolveMultiple` (`|MakeArray` (`self.OrbitingPlatform10`) (`self.OrbitingPlatform11`) (`self.OrbitingPlatform9`)) (`SceneComponent.RelativeLocation` (`self.OrbitingPlatform2`)) false)
  (`self.OrbitSolveMultiple` (`|MakeArray` (`self.OrbitingPlatform7`) (`self.OrbitingPlatform8`) (`self.OrbitingPlatform6`)) (`SceneComponent.RelativeLocation` (`self.OrbitingPlatform1`)) false))

(fn `UserConstructionScript`)