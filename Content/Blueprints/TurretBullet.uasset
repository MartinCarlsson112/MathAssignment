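; Pooled projectile fired by a turret that damages Spaceship actors it overlaps.
; Fire places and activates the bullet, moves it each Tick by a constant velocity without sweeping, and starts a lifetime timer.
; On a damageable Spaceship overlap or timer expiry, it hides, disables collision and tick, and returns itself to its Shooter by index.
; Damage goes through DamageableInterface, crediting the Shooter's owner.
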(event `self.ReceiveTick`
  (params (DeltaSeconds :type "Float (single-precision)"))
  (`self.K2_SetActorLocation` (+ (`self.K2_GetActorLocation`) (* (`self.Velocity`) DeltaSeconds))))

(event `self.StaticMesh.OnComponentHit`
  (params (HitComponent :type "PrimitiveComponent Object Reference") (OtherActor :type "Actor Object Reference") (OtherComp :type "PrimitiveComponent Object Reference") (NormalImpulse :type "Vector Structure") (Hit :type "HitResult Structure (by ref)")))

(event `self.StaticMesh.OnComponentBeginOverlap`
  (params (OverlappedComponent :type "PrimitiveComponent Object Reference") (OtherActor :type "Actor Object Reference") (OtherComp :type "PrimitiveComponent Object Reference") (OtherBodyIndex :type Integer) (bFromSweep :type Boolean) (SweepResult :type "HitResult Structure (by ref)"))
  (if (and (== (`GameplayStatics.GetObjectClass` OtherActor) "/Game/Blueprints/Spaceship.Spaceship_C") (`KismetSystemLibrary.DoesImplementInterface` OtherActor "/Game/Blueprints/DamageableInterface.DamageableInterface_C"))
    (message `/Game/Blueprints/DamageableInterface.ReceiveDamage` OtherActor (`self.BulletDamage`) (`ActorComponent.GetOwner` (`self.Shooter`)))
    (`self.Expire`)))

(fn `ActivateBullet`
  (`SceneComponent.SetHiddenInGame` (`self.StaticMesh`) false false)
  (`PrimitiveComponent.SetCollisionEnabled` (`self.StaticMesh`) "QueryAndPhysics")
  (`self.SetActorTickEnabled` true))

(fn `DeactivateBullet`
  (`SceneComponent.SetHiddenInGame` (`self.StaticMesh`) true false)
  (`PrimitiveComponent.SetCollisionEnabled` (`self.StaticMesh`) "NoCollision")
  (`self.SetActorTickEnabled` false))

(fn `Expire`
  (`self.DeactivateBullet`)
  (`/Game/Blueprints/Turret.ReturnBullet` (`self.Shooter`) (`self.BulletIndex`))
  (`KismetSystemLibrary.K2_ClearAndInvalidateTimerHandle` (`self.LifetimeHandle`)))

(fn `Fire`
  (params (StartPosition :type "Vector Structure") (Direction :type "Vector Structure") (Speed :type "Float (double-precision)"))
  (`self.K2_SetActorLocation` StartPosition)
  (`self.ActivateBullet`)
  (set `self.Velocity` (* Direction Speed))
  (bind _returnvalue (`KismetSystemLibrary.K2_SetTimer` null "Expire" (`self.Lifetime`)))
  (set `self.LifetimeHandle` _returnvalue))

(fn `Initialize`
  (params (Index :type Integer) (Shooter :type "/Game/Blueprints/Turret Object Reference"))
  (set `self.BulletIndex` Index)
  (set `self.Shooter` Shooter))

(fn `UserConstructionScript`)