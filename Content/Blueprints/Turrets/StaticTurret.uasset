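; Static turret that detects targets with two shooter components and takes damage until destroyed.
; Tick runs detection on both shooters and snaps Body toward RightShooter's target, without interpolation.
; Each shooter's FoundTarget starts a looping timer that fires the opposite shooter, with one delayed to alternate shots; LostTarget leaves timers running.
; Non-lethal damage makes both shooters aggro the attacker; zero health destroys them and the actor.
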(event `self.ReceiveBeginPlay`
  (set `self.Health` (`self.MaxHealth`)))

(event `self.ReceiveTick`
  (params (DeltaSeconds :type "Float (single-precision)"))
  (bind _body (`self.Body`))
  (`/Game/Blueprints/Turret.Detect` (`self.RightShooter`))
  (`/Game/Blueprints/Turret.Detect` (`self.LeftShooter`))
  (`/Engine/EditorBlueprintResources/StandardMacros.IsValid` (`/Game/Blueprints/Turret.Target` (`self.RightShooter`))
    (:`Is Valid`
      (`SceneComponent.K2_SetWorldRotation` _body (`KismetMathLibrary.FindLookAtRotation` (`SceneComponent.K2_GetComponentLocation` _body) (`self.K2_GetActorLocation` (`/Game/Blueprints/Turret.Target` (`self.RightShooter`)))) false false))))

(event `self.RightShooter.FoundTarget`
  (`KismetSystemLibrary.K2_SetTimerDelegate` (delegate `LeftFire`) (* (`self.ShootCooldown`) 2.0) true))

(event `LeftFire`
  (`/Game/Blueprints/Turret.Fire` (`self.LeftShooter`)))

(event `self.RightShooter.TargetSwitched`)

(event `self.RightShooter.LostTarget`)

(event `self.LeftShooter.FoundTarget`
  (`KismetSystemLibrary.K2_SetTimerDelegate` (delegate `RightFire`) (* (`self.ShootCooldown`) 2.0) true (`self.ShootCooldown`)))

(event `RightFire`
  (`/Game/Blueprints/Turret.Fire` (`self.RightShooter`)))

(event `self.LeftShooter.TargetSwitched`)

(event `self.LeftShooter.LostTarget`)

(event `self.RightShooter.Destroyed`
  (`KismetSystemLibrary.PrintString` "destroyed"))

(event `self.LeftShooter.Destroyed`
  (`KismetSystemLibrary.PrintString` "destroyed"))

(fn `Destroy`
  (`/Game/Blueprints/Turret.Destroy` (`self.RightShooter`))
  (`/Game/Blueprints/Turret.Destroy` (`self.LeftShooter`)))

(fn `ReceiveDamage`
  (params (DamageAmount :type "Float (double-precision)") (Shooter :type "Actor Object Reference"))
  (returns (DamageDealt :type "Float (double-precision)"))
  (`KismetSystemLibrary.PrintString` "Took damage")
  (bind _output_get (set `self.Health` (- (`self.Health`) DamageAmount)))
  (if (<= _output_get 0.0)
    (`self.Destroy`)
    (`self.K2_DestroyActor`)
    (return DamageAmount)
    (else
      (`/Game/Blueprints/Turret.AggroTarget` (`self.LeftShooter`) Shooter)
      (`/Game/Blueprints/Turret.AggroTarget` (`self.RightShooter`) Shooter)
      (return DamageAmount))))

(fn `UserConstructionScript`)