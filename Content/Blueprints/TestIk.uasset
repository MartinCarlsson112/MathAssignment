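; TestIk is a test Blueprint that exercises an inverse kinematics solver on a five-bone chain.
; BeginPlay builds and stores the chain from IK through IK4, starting at IK.
; Each Tick runs a FABRIK solve on that chain toward TargetPoint.
; A CCD solver call with a threshold and step limit is also present but disconnected, so it never runs.
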(event `self.ReceiveBeginPlay`
  (bind _returnvalue (`IKSolver.CreateIKChain` (`|MakeArray` (`self.IK`) (`self.IK1`) (`self.IK2`) (`self.IK3`) (`self.IK4`)) (`self.IK`)))
  (set `self.IkChain` _returnvalue))

(event `self.ReceiveTick`
  (params (DeltaSeconds :type "Float (single-precision)"))
  (`IKSolver.SolveIKChainFABRIK` (`self.IkChain`) (`self.Target Point`)))

(fn `UserConstructionScript`)