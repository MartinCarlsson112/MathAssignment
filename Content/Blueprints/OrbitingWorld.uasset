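; OrbitingWorld is an actor that animates ten orbit components circling a shared pivot at the zero vector.
; Each tick, OrbitSolveMultipleComponents receives the components, the pivot and the current game time to solve their orbits.
; RotationSolve then takes the same components with a small fixed speed vector and the frame delta to spin them.
; The construction script is empty, so all behavior lives in Tick.
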(event `self.ReceiveTick`
  (params (DeltaSeconds :type "Float (single-precision)"))
  (bind _array (`|MakeArray` (`self.Orbit`) (`self.Orbit1`) (`self.Orbit2`) (`self.Orbit3`) (`self.Orbit4`) (`self.Orbit5`) (`self.Orbit6`) (`self.Orbit7`) (`self.Orbit8`) (`self.Orbit9`)))
  (`OrbitSolver.OrbitSolveMultipleComponents` _array (0.0 0.0 0.0) (`GameplayStatics.GetTimeSeconds`))
  (`OrbitSolver.RotationSolve` _array (0.001 0.001 0.0001) DeltaSeconds))

(fn `UserConstructionScript`)