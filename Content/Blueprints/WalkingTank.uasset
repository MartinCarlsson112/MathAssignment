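; Eight-legged walking tank actor that circles its spawn point on a solved orbit while its turret detects and fires.
; Each tick, a step solver with a randomized threshold relocates world-space animation targets when legs need to step.
; Per-leg timelines interpolate IK targets toward them with a step-height offset, and FABRIK solves each chain.
; The construction script also builds and solves the leg chains.
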(event `self.ReceiveBeginPlay`
  (`self.AddIKComponent` (`self.LeftFrontLeg`) (`self.LeftFrontTarget`) (`self.LeftFrontPole`) (`self.LeftFrontAnimationTarget`))
  (`self.AddIKComponent` (`self.LeftMiddle1Leg`) (`self.LeftMiddle1Target`) (`self.LeftMiddle1Pole`) (`self.LeftMiddle1AnimationTarget`))
  (`self.AddIKComponent` (`self.LeftMiddle2Leg`) (`self.LeftMiddle2Target`) (`self.LeftMiddle2Pole`) (`self.LeftMiddle2AnimationTarget`))
  (`self.AddIKComponent` (`self.LeftBackLeg`) (`self.LeftBackTarget`) (`self.LeftBackPole`) (`self.LeftBackAnimationTarget`))
  (`self.AddIKComponent` (`self.RightFrontLeg`) (`self.RightFrontTarget`) (`self.RightFrontPole`) (`self.RightFrontAnimationTarget`))
  (`self.AddIKComponent` (`self.RightMiddle1Leg`) (`self.RightMiddle1Target`) (`self.RightMiddle1Pole`) (`self.RightMiddle1AnimationTarget`))
  (`self.AddIKComponent` (`self.RightMiddle2Leg`) (`self.RightMiddle2Target`) (`self.RightMiddle2Pole`) (`self.RightMiddle2AnimationTarget`))
  (`self.AddIKComponent` (`self.RightBackLeg`) (`self.RightBackTarget`) (`self.RightBackPole`) (`self.RightBackAnimationTarget`))
  (set `self.Orbit Pivot` (`self.K2_GetActorLocation`))
  (`TimelineComponent.SetTimelineLength` (`self.Timeline_6`) (`self.AnimationSpeed`))
  (`TimelineComponent.SetTimelineLength` (`self.Timeline_4`) (`self.AnimationSpeed`))
  (`TimelineComponent.SetTimelineLength` (`self.Timeline_3`) (`self.AnimationSpeed`))
  (`TimelineComponent.SetTimelineLength` (`self.Timeline_7`) (`self.AnimationSpeed`))
  (`TimelineComponent.SetTimelineLength` (`self.Timeline_1`) (`self.AnimationSpeed`))
  (`TimelineComponent.SetTimelineLength` (`self.Timeline_0`) (`self.AnimationSpeed`))
  (`TimelineComponent.SetTimelineLength` (`self.Timeline_5`) (`self.AnimationSpeed`))
  (`TimelineComponent.SetTimelineLength` (`self.Timeline_2`) (`self.AnimationSpeed`)))

(event `self.ReceiveTick`
  (params (DeltaSeconds :type "Float (single-precision)"))
  (bind _turret (`self.Turret`))
  (for (_array_element _array_index) (`self.LegComponents`)
    ;[1 1 1] Walking animation, Excuse the mess
    (bind (_newposition _target) (`self.StepSolver` _array_element (`|GetArrayItem` (`self.AnimationTargets`) _array_index) (`|GetArrayItem` (`self.LegPoles`) _array_index))
      (:`Step`
        (switch `int` _array_index
          (:`0`
            (`SceneComponent.K2_SetWorldLocation` _target _newposition false false)
            (bind (_direction _newtrack_0) (`Timeline|Timeline_6` :!via `PlayFromStart`)
              (:`Update`
                (`self.InterpLegPosition` 0 _newtrack_0))))
          (:`1`
            (`SceneComponent.K2_SetWorldLocation` _target _newposition false false)
            (bind (_direction_2 _newtrack_0_2) (`Timeline|Timeline_0` :!via `PlayFromStart`)
              (:`Update`
                (`self.InterpLegPosition` 1 _newtrack_0_2))))
          (:`2`
            (`SceneComponent.K2_SetWorldLocation` _target _newposition false false)
            (bind (_direction_3 _newtrack_0_3) (`Timeline|Timeline_7` :!via `PlayFromStart`)
              (:`Update`
                (`self.InterpLegPosition` 2 _newtrack_0_3))))
          (:`3`
            (`SceneComponent.K2_SetWorldLocation` _target _newposition false false)
            (bind (_direction_4 _newtrack_0_4) (`Timeline|Timeline_1` :!via `PlayFromStart`)
              (:`Update`
                (`self.InterpLegPosition` 3 _newtrack_0_4))))
          (:`4`
            (`SceneComponent.K2_SetWorldLocation` _target _newposition false false)
            (bind (_direction_5 _newtrack_0_5) (`Timeline|Timeline_2` :!via `PlayFromStart`)
              (:`Update`
                (`self.InterpLegPosition` 4 _newtrack_0_5))))
          (:`5`
            (`SceneComponent.K2_SetWorldLocation` _target _newposition false false)
            (bind (_direction_6 _newtrack_0_6) (`Timeline|Timeline_3` :!via `PlayFromStart`)
              (:`Update`
                (`self.InterpLegPosition` 5 _newtrack_0_6))))
          (:`6`
            (`SceneComponent.K2_SetWorldLocation` _target _newposition false false)
            (bind (_direction_7 _newtrack_0_7) (`Timeline|Timeline_4` :!via `PlayFromStart`)
              (:`Update`
                (`self.InterpLegPosition` 6 _newtrack_0_7))))
          (:`7`
            (`SceneComponent.K2_SetWorldLocation` _target _newposition false false)
            (bind (_direction_8 _newtrack_0_8) (`Timeline|Timeline_5` :!via `PlayFromStart`)
              (:`Update`
                (`self.InterpLegPosition` 7 _newtrack_0_8))))))))
  (for (_array_element_2 _array_index_2) (`self.Legs`)
    (`IKSolver.SolveIKChainFABRIK` _array_element_2 (`|GetArrayItem` (`self.Target Points`) _array_index_2)))
  (bind _returnvalue (`OrbitSolver.SolveOrbit` (make `OrbitSolverData` (1000.0 0.0 0.0) (0.0 0.0 0.0) (12.5 0.0 0.0)) (`self.Orbit Pivot`) (`GameplayStatics.GetTimeSeconds`)))
  (`self.K2_SetActorLocation` _returnvalue)
  (`KismetSystemLibrary.Delay` 0.1)
  (`/Game/Blueprints/Turret.Detect` _turret)
  (`/Game/Blueprints/Turret.Fire` _turret))

(fn `UserConstructionScript`
  (`self.ConstructIKChainComponent` (`self.RightFrontLeg`) (`self.RightFrontTarget`))
  (`self.ConstructIKChainComponent` (`self.RightBackLeg`) (`self.RightBackTarget`))
  (`self.ConstructIKChainComponent` (`self.RightMiddle1Leg`) (`self.RightMiddle1Target`))
  (`self.ConstructIKChainComponent` (`self.RightMiddle2Leg`) (`self.RightMiddle2Target`))
  (`self.ConstructIKChainComponent` (`self.LeftFrontLeg`) (`self.LeftFrontTarget`))
  (`self.ConstructIKChainComponent` (`self.LeftMiddle1Leg`) (`self.LeftMiddle1Target`))
  (`self.ConstructIKChainComponent` (`self.LeftMiddle2Leg`) (`self.LeftMiddle2Target`))
  (`self.ConstructIKChainComponent` (`self.LeftBackLeg`) (`self.LeftBackTarget`)))